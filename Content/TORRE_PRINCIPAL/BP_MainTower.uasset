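; BP_MainTower is the main tower actor, which tracks its health and shows it on screen.
; On BeginPlay it creates a WBP_MainTowerHealth widget, adds it to the viewport and pushes the starting health values.
; Its custom TakeDamage function subtracts damage, clamps health between zero and the maximum and refreshes the widget.
; The zero-health check leads to no logic, so depletion has no effect here.
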(event EventBeginPlay
  (bind _returnvalue (UserInterface|CreateWidget "/Game/Fab/Megascans/3D/Japanese_Metal_Lantern_vfvjccaqx/Low/WBP_MainTowerHealth.WBP_MainTowerHealth_C"))
  (bind _output_get (Variables|Default|SetHealthUI _returnvalue))
  (UserInterface|Viewport|AddtoViewport _output_get 0)
  (Default|UpdateHealth _output_get (Variables|Default|GetCurrentHealth) (Variables|Default|GetMaxHealth)))

(event Collision|EventActorBeginOverlap
  (params (OtherActor :type Actor%20Object%20Reference)))

(event EventTick
  (params (DeltaSeconds :type Float%20%28single-precision%29)))

(fn ConstructionScript)

(fn TakeDamage
  (params (DamageAmount :type Float%20%28double-precision%29))
  (Variables|Default|SetCurrentHealth (Math|Float|Clamp(Float) (- (Variables|Default|GetCurrentHealth) DamageAmount) 0.0 (Variables|Default|GetMaxHealth)))
  (Default|UpdateHealth (Variables|Default|GetHealthUI) (Variables|Default|GetCurrentHealth) (Variables|Default|GetMaxHealth))
  (if (<= (Variables|Default|GetCurrentHealth) 0.0)
    _))