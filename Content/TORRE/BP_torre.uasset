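; BP_torre is a tower actor that detects Bp_Unit troops inside a spherical range.
; The construction script sizes RangoSphere from the Rangoo variable.
; Each Tick rebuilds TropaEnRango from the sphere's overlapping units and prints whether any are present.
; Begin overlap only prints a debug message, end overlap also removes the unit from the array, and no attack logic exists yet.
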(event OnComponentBeginOverlap(RangoSphere)
  (params (OverlappedComponent :type Primitive%20Component%20Object%20Reference) (OtherActor :type Actor%20Object%20Reference) (OtherComp :type Primitive%20Component%20Object%20Reference) (OtherBodyIndex :type Integer) (bFromSweep :type Boolean) (SweepResult :type Hit%20Result%20Structure%20%28by%20ref%29))
  (Development|PrintString "ENTRO UNA TROPA!!!"))

(event OnComponentEndOverlap(RangoSphere)
  (params (OverlappedComponent :type Primitive%20Component%20Object%20Reference) (OtherActor :type Actor%20Object%20Reference) (OtherComp :type Primitive%20Component%20Object%20Reference) (OtherBodyIndex :type Integer))
  (bind _asbp_unit (Utilities|Casting|CastToBp_Unit OtherActor))
  (Utilities|Array|RemoveItem (Variables|Default|GetTropaEnRango) _asbp_unit)
  (Development|PrintString "SALIO TROPA!!!"))

(event EventBeginPlay)

(event Collision|EventActorBeginOverlap
  (params (OtherActor :type Actor%20Object%20Reference)))

(event EventTick
  (params (DeltaSeconds :type Float%20%28single-precision%29))
  (bind _output_get (Variables|Default|SetTropaEnRango (Collision|GetOverlappingActors (Variables|Default|GetRangoSphere) "/Game/TROPAS/Bp_Unit.Bp_Unit_C" :!class /Script/Engine.PrimitiveComponent)))
  (if (> (Utilities|Array|Length _output_get) 0)
    (Development|PrintString "HAY TROPA")
    (else
      (Development|PrintString "NO HAY TROPA"))))

(fn ConstructionScript
  (Components|Sphere|SetSphereRadius (Variables|Default|GetRangoSphere) (Variables|Default|GetRangoo) true))