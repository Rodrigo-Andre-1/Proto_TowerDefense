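; Troop unit that walks a generated grid path and damages towers at its end, with a flipbook chosen by unit type.
; BeginPlay gets a non-diagonal path from Generator, teleports to its last tile and stores waypoints at actor height, drawing debug spheres.
; Tick steps backwards through them, then damages TowerRef and the main tower and self-destructs.
; AnyDamage sets health to damage minus MaxHealth, destroying the unit at zero or below.
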(event Custom|StartPaths
  (Variables|Default|SetcurrentIndex (Utilities|Array|LastIndex (Variables|Default|GetTargetLocation)))
  (Variables|Default|SetisMoving true))

(event EventBeginPlay
  ;[0 0 0 0.5] Tratar de obtener path de un generator
  (bind _returnvalue (Actor|GetActorOfClass "/Game/TORRE_PRINCIPAL/BP_MainTower.BP_MainTower_C"))
  (Variables|MainTower|SetMainTowerRef _returnvalue)
  (bind _generator (Variables|Default|Getgenerator)
    (:then
      ;[0 0 0 0.5] Si hay un path armamos el spline y lo iniciamos
      (CallFunction|BuildSplinePath (.OutPath (Default|FindPath _generator (Utilities|Struct|MakeST_PathInfo (Variables|Default|GetIn%20Path%20Start) (Variables|Default|GetIn%20Path%20End) false))))
      (CallFunction|StartPaths))
    (:else
      (Development|PrintString "FailedToObtain" true true "(R=1.000000,G=0.000000,B=0.000000,A=1.000000)"))))

(event Game|Damage|EventAnyDamage
  (params (Damage :type Float%20%28single-precision%29) (DamageType :type Damage%20Type%20Object%20Reference) (InstigatedBy :type Controller%20Object%20Reference) (DamageCauser :type Actor%20Object%20Reference))
  (Variables|Default|SetCurrentHealth (- Damage (Variables|Default|GetMaxHealth)))
  (if (<= (Variables|Default|GetCurrentHealth) 0.0)
    (Actor|DestroyActor)))

(event EventTick
  (params (DeltaSeconds :type Float%20%28single-precision%29))
  (CallFunction|TravelPath))

(fn ConstructionScript
  (Sprite|SetFlipbook (Variables|Default|GetPaperFlipbook) (Utilities|Select :Index (Variables|Default|GetUnitType) :NewEnumerator0 0 :NewEnumerator1 0 :NewEnumerator2 0 :NewEnumerator3 0 :NewEnumerator4 0)))

(fn BuildSplinePath
  (params (InPath :type Array%20of%20BP%20Tile%20Object%20References))
  (bind _returnvalue (Utilities|Array|LastIndex InPath))
  (bind _output (Utilities|Array|Get(acopy) InPath _returnvalue))
  (bind _tile (Variables|/Game/MAPAS/BLUEPRINTS/BP_Tile.BP_Tile_C|GetTile _output))
  (bind _returnvalue_2 (Transformation|GetWorldLocation _tile))
  (Transformation|SetActorLocation (Math|Vector|MakeVector (.x _returnvalue_2) (.y _returnvalue_2) (.z (Transformation|GetActorLocation))) true true)
  (for _array_element InPath
    (bind _returnvalue_3 (Utilities|Array|Add (Variables|Default|GetTargetLocation) (Math|Vector|MakeVector (.x (Transformation|GetActorLocation _array_element)) (.y (Transformation|GetActorLocation _array_element)) (.z (Transformation|GetActorLocation)))))
    (Rendering|Debug|DrawDebugSphere (Utilities|Array|Get(acopy) (Variables|Default|GetTargetLocation) _returnvalue_3) 15.0 12 "(R=1.000000,G=0.105790,B=0.990712,A=1.000000)" 99.0)))

(fn TravelPath
  (bind _returnvalue (Transformation|GetActorLocation))
  (bind _towerref (Variables|Default|GetTowerRef))
  (if (Variables|Default|GetisMoving)
    (bind _output_get (Variables|Default|SettargetPoint (Utilities|Array|Get(acopy) (Variables|Default|GetTargetLocation) (Variables|Default|GetcurrentIndex))))
    ;[0 0 0 0.5] Si la distance entre el actor y el punto objetivo es menor que stopDistance seguir moviendose, de lo contrario llegó al puno (poner stopDistance con un valor de al menos 1)
    (if (<= (Math|Vector|Distance(Vector) _output_get (Transformation|GetActorLocation)) (Variables|Default|GetstopDistance))
      ;[0 0 0 0.5] Setar el current Index por el siguiente punto en el arreglo de targetLocations
      (bind _result (Math|Integer|DecrementInt (Variables|Default|GetcurrentIndex))
        (:%20%20
          (bind _output_get_2 (Variables|Default|SetcurrentIndex _result))
          (if (<= _output_get_2 -1)
            (Variables|Default|SetisMoving false)
            (Utilities|IsValid _towerref
              (:Is%20Valid
                (Default|ReceiveTowerDamage _towerref (Variables|Default|GetDamageToTower)))
              (:Is%20Not%20Valid
                _))
            (CallFunction|DamageMainTower)
            (Actor|DestroyActor))))
      (else
        ;[0 0 0 0.5] Mover el actor al punto actual
        (Variables|Default|Setdirection (Math|Vector|Normalize (- (Variables|Default|GettargetPoint) _returnvalue)))
        (Transformation|SetActorLocation (+ _returnvalue (* (* (Variables|Default|Getdirection) (Variables|Default|GetmovementSpeed)) (Utilities|Time|GetWorldDeltaSeconds))) false false)))))

(fn DamageMainTower
  (bind _maintowerref (Variables|MainTower|GetMainTowerRef))
  (Utilities|IsValid _maintowerref
    (:Is%20Valid
      (Default|TakeDamage _maintowerref (Variables|MainTower|GetDamageToMainTower)))))