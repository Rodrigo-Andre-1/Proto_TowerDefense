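; Player controller for board-style path selection by mouse click, active while the possessed BP_Character is not flagged as controlling the character.
; It adds the general Enhanced Input context, then traces under the cursor for actors implementing BPI_Interactable.
; Clicks pick a start and an end actor, toggle their state through interact messages and request a path between them.
; Clicking the start again deselects it, while clicking another actor after a completed pair begins a new selection.
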(event Input|EnhancedActionEvents|EnhancedInputActionIA_Click
  (params (ActionValue :type Boolean) (ElapsedSeconds :type Float%20%28double-precision%29) (TriggeredSeconds :type Float%20%28double-precision%29) (InputAction :type Input%20Action%20Object%20Reference :default "/Game/PLAYER/CAMERA_ESTATICA/BLUEPRINTS/CamaraEstatica/IA_Click.IA_Click"))
  (bind (_success _clickedactor) (CallFunction|GetClickedActor))
  (bind _asbp_character (Utilities|Casting|CastToBP_Character (Pawn|GetControlledPawn)))
  (if (not (Variables|/Game/PLAYER/CHARACTER/BP_Character.BP_Character_C|GetIsControlingCharacter _asbp_character))
    (Development|PrintString "Click")
    (Utilities|FlowControl|Sequence
      (:then_0
        (Variables|Default|GetStartPath
          (:then
            (Variables|Default|GetEndPath
              (:then
                (Class|BPIInteractable|OnInteract(Message) (Variables|Default|GetStartPath) "NewEnumerator0")
                (Class|BPIInteractable|OnInteract(Message) (Variables|Default|GetEndPath) "NewEnumerator0"))
              (:else)))
          (:else)))
      (:then_1
        (if _success
          (if (== _clickedactor (Variables|Default|GetStartPath))
            (Class|BPIInteractable|OnInteract(Message) (Variables|Default|GetStartPath) "NewEnumerator0")
            (Variables|Default|SetStartPath 0)
            (else
              (Variables|Default|GetStartPath
                (:then
                  (Variables|Default|GetEndPath
                    (:then
                      (bind _output_get (Variables|Default|SetStartPath _clickedactor :!label _label))
                      (Class|BPIInteractable|OnInteract(Message) _output_get "NewEnumerator1")
                      (Variables|Default|SetEndPath 0))
                    (:else
                      (bind _output_get_2 (Variables|Default|SetEndPath _clickedactor))
                      (Class|BPIInteractable|OnInteract(Message) _output_get_2 "NewEnumerator1")
                      (Default|CallFindPathto (Variables|Default|GetStartPath) (Variables|Default|GetEndPath)))))
                (:else
                  (goto _label))))))))))

(event EventBeginPlay
  (CallFunction|SetupInput))

(fn ConstructionScript)

(fn SetupInput
  (bind _returnvalue (PlayerController|LocalPlayerSubsystems|GetEnhancedInputLocalPlayerSubsystem))
  (Utilities|IsValid _returnvalue
    (:Is%20Valid
      (Input|AddMappingContext _returnvalue "/Game/PLAYER/CAMERA_ESTATICA/BLUEPRINTS/CamaraEstatica/IMC_General.IMC_General" 0 "(bIgnoreAllPressedKeysUntilRelease=True,bForceImmediately=False,bNotifyUserSettings=False)"))))

(fn GetClickedActor
  (bind (_hitresult _returnvalue) (Game|Player|GetHitResultUnderCursorbyChannel "TraceTypeQuery3" true))
  (bind _hitactor (Collision|BreakHitResult _hitresult))
  (Development|PrintString (Utilities|GetDisplayName _hitactor))
  (return (and _returnvalue (Utilities|DoesObjectImplementInterface _hitactor "/Game/PLAYER/CAMERA_ESTATICA/BLUEPRINTS/CamaraEstatica/BPI_Interactable.BPI_Interactable_C")) _hitactor))