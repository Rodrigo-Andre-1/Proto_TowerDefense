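; BP_Player1BoardController is a player controller that handles click selection of interactable actors, likely on a game board.
; On BeginPlay it adds the general Enhanced Input mapping context.
; Each click traces under the cursor for an actor implementing BPI_Interactable, first sending a deselect interface message to the current selection.
; Clicking the selected actor again clears it; clicking another interactable stores and selects it, with debug prints along the way.
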(event Input|EnhancedActionEvents|EnhancedInputActionIA_Click
  (params (ActionValue :type Boolean) (ElapsedSeconds :type Float%20%28double-precision%29) (TriggeredSeconds :type Float%20%28double-precision%29) (InputAction :type Input%20Action%20Object%20Reference :default "/Game/PLAYER/BLUEPRINTS/IA_Click.IA_Click"))
  (bind (_success _clickedactor) (CallFunction|GetClickedActor))
  (:Triggered
    (Development|PrintString "Click")
    (Utilities|FlowControl|Sequence
      (:then_0
        (bind _selectedactor (Variables|Default|GetSelectedActor)
          (:then
            (Class|BPIInteractable|OnInteract(Message) _selectedactor false))
          (:else)))
      (:then_1
        (if _success
          (if (== _clickedactor (Variables|Default|GetSelectedActor))
            (Variables|Default|SetSelectedActor 0)
            (else
              (bind _output_get (Variables|Default|SetSelectedActor _clickedactor))
              (Class|BPIInteractable|OnInteract(Message) _output_get true))))))))

(event EventBeginPlay
  (CallFunction|SetupInput))

(fn ConstructionScript)

(fn SetupInput
  (bind _returnvalue (PlayerController|LocalPlayerSubsystems|GetEnhancedInputLocalPlayerSubsystem))
  (Utilities|IsValid _returnvalue
    (:Is%20Valid
      (Input|AddMappingContext _returnvalue "/Game/PLAYER/BLUEPRINTS/IMC_General.IMC_General" 0 "(bIgnoreAllPressedKeysUntilRelease=True,bForceImmediately=False,bNotifyUserSettings=False)"))))

(fn GetClickedActor
  (bind (_hitresult _returnvalue) (Game|Player|GetHitResultUnderCursorbyChannel "TraceTypeQuery3" true))
  (bind _hitactor (Collision|BreakHitResult _hitresult))
  (Development|PrintString (Utilities|GetDisplayName _hitactor))
  (return (and _returnvalue (Utilities|DoesObjectImplementInterface _hitactor "/Game/PLAYER/BLUEPRINTS/BPI_Interactable.BPI_Interactable_C")) _hitactor))