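; Player character for a tile-board game that selects non-path tiles for a tower menu and toggles its view with a board camera.
; Tick traces downward ahead of the character to target a BP_Tile; the select input highlights it and opens the tower widget with focus.
; The switch input blends cameras and gates movement.
; BeginPlay sets up input and the money widget; PowerUps adds money, with other types only printing.
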(event Input|EnhancedActionEvents|EnhancedInputActionIA_CharacterMove
  (params (ActionValue :type Vector%202D%20Structure) (ElapsedSeconds :type Float%20%28double-precision%29) (TriggeredSeconds :type Float%20%28double-precision%29) (InputAction :type Input%20Action%20Object%20Reference :default "/Game/PLAYER/CHARACTER/IA_CharacterMove.IA_CharacterMove"))
  (bind (_x _y) (Math|Vector2D|BreakVector2D ActionValue))
  ;[0.15 0.15 0.15 0.5] Movimiento
  (if (Variables|Default|GetIsControlingCharacter)
    (Pawn|Input|AddMovementInput (Math|Vector|GetRightVector (Math|Rotator|MakeRotator 0.0 0.0 (.Yaw (Math|Rotator|BreakRotator (Pawn|GetControlRotation :!class /Script/Engine.Pawn))))) _x false)
    (Pawn|Input|AddMovementInput (Math|Vector|GetForwardVector (Math|Rotator|MakeRotator 0.0 0.0 (.Yaw (Math|Rotator|BreakRotator (Pawn|GetControlRotation :!class /Script/Engine.Pawn))))) _y false)))

(event Input|EnhancedActionEvents|EnhancedInputActionIA_Switch
  (params (ActionValue :type Boolean) (ElapsedSeconds :type Float%20%28double-precision%29) (TriggeredSeconds :type Float%20%28double-precision%29) (InputAction :type Input%20Action%20Object%20Reference :default "/Game/PLAYER/SWITCH/IA_Switch.IA_Switch"))
  (bind _returnvalue (Game|GetPlayerController 0))
  ;[0.15 0.15 0.15 0.5] Camviar a Tablero
  (:Started
    (if (Variables|Default|GetIsControlingCharacter)
      (Game|Player|SetViewTargetwithBlend _returnvalue (Variables|Default|GetBoardCamera) 0.5 "VTBlend_Linear" 0.0 false)
      (Variables|Default|SetIsControlingCharacter false)
      (else
        (Game|Player|SetViewTargetwithBlend _returnvalue self 0.5 "VTBlend_Linear" 0.0 false)
        (Variables|Default|SetIsControlingCharacter true)))))

(event Input|EnhancedActionEvents|EnhancedInputActionIA_SelectTIle
  (params (ActionValue :type Boolean) (ElapsedSeconds :type Float%20%28double-precision%29) (TriggeredSeconds :type Float%20%28double-precision%29) (InputAction :type Input%20Action%20Object%20Reference :default "/Game/PLAYER/CHARACTER/IA_SelectTIle.IA_SelectTIle"))
  (bind _returnvalue (Game|GetPlayerController 0))
  (bind _targetedtile (Variables|Default|GetTargetedTIle))
  ;[0.15 0.15 0.15 0.5] Seleccionar TIle
  (:Started
    (Utilities|IsValid (Variables|Default|GetSelectedTile)
      (:Is%20Valid
        (Default|SetTileSelectedColor (Variables|Default|GetSelectedTile) false))
      (:Is%20Not%20Valid
        _))
    (Utilities|IsValid _targetedtile
      (:Is%20Valid
        (bind _asbp_tile (Utilities|Casting|CastToBP_Tile _targetedtile))
        (if (not (Variables|/Game/MAPAS/BLUEPRINTS/BP_Tile.BP_Tile_C|GetIsPath _asbp_tile))
          (Default|SetTileSelectedColor _asbp_tile true)
          (Variables|Default|SetSelectedTile _asbp_tile)
          (Development|PrintString (Utilities|String|Append "TILE 
" "R: " (Utilities|String|ToString(Integer) (.Row (Utilities|Struct|BreakST_Coordinates (Variables|/Game/MAPAS/BLUEPRINTS/BP_Tile.BP_Tile_C|GetCoordinates _asbp_tile)))) " 
C: " (Utilities|String|ToString(Integer) (.Column (Utilities|Struct|BreakST_Coordinates (Variables|/Game/MAPAS/BLUEPRINTS/BP_Tile.BP_Tile_C|GetCoordinates _asbp_tile)))) " 
SELECCIONADA") true true "(R=1.000000,G=0.981936,B=0.000000,A=1.000000)" 3.0)
          (Utilities|IsValid (Variables|Default|GetMenuActual)
            (:Is%20Valid
              (Widget|RemovefromParent (Variables|Default|GetMenuActual))
              (bind _asbp_tile_2 (Utilities|Casting|CastToBP_Tile (Variables|Default|GetTargetedTIle)))
              (if (not (Variables|/Game/MAPAS/BLUEPRINTS/BP_Tile.BP_Tile_C|GetIsPath _asbp_tile_2))
                (bind _returnvalue_2 (UserInterface|CreateWidget "/Game/UI/MenuTorres.MenuTorres_C" 0 _asbp_tile self :!label _label))
                (bind _output_get (Variables|Default|SetMenuActual _returnvalue_2))
                (UserInterface|Viewport|AddtoViewport _output_get 0)
                (Input|SetInputModeGameOnly _returnvalue false)
                (Class|Widget|SetUserFocus (Variables|/Game/UI/MenuTorres.MenuTorres_C|GetBtn_Torre1 (Variables|Default|GetMenuActual)) _returnvalue)
                (Variables|/Script/Engine.PlayerController|SetbShowMouseCursor (Game|GetPlayerController 0) false)))
            (:Is%20Not%20Valid
              (goto _label))))))))

(event EventBeginPlay
  (bind _returnvalue (Game|GetPlayerController 0))
  ;[0.15 0.15 0.15 0.5] Camviar a Tablero
  (Variables|/Script/Engine.PlayerController|SetbShowMouseCursor _returnvalue false)
  (Variables|/Script/Engine.PlayerController|SetbEnableClickEvents _returnvalue false)
  (Variables|/Script/Engine.PlayerController|SetbEnableMouseOverEvents _returnvalue false)
  (Input|AddMappingContext (PlayerController|LocalPlayerSubsystems|GetEnhancedInputLocalPlayerSubsystem _returnvalue) "/Game/PLAYER/CHARACTER/IMC_CharacterController.IMC_CharacterController" 1 "(bIgnoreAllPressedKeysUntilRelease=True,bForceImmediately=False,bNotifyUserSettings=False)")
  (Game|Player|SetViewTargetwithBlend _returnvalue self 0.0 "VTBlend_Linear" 0.0 false)
  (bind _returnvalue_2 (Actor|GetActorOfClass "/Script/Engine.CameraActor"))
  (Variables|Default|SetBoardCamera _returnvalue_2)
  (bind _returnvalue_3 (UserInterface|CreateWidget "/Game/UI/WPB_Dinerou.WPB_Dinerou_C" 0 self))
  (UserInterface|Viewport|AddtoViewport _returnvalue_3 0))

(event Collision|EventActorBeginOverlap
  (params (OtherActor :type Actor%20Object%20Reference)))

(event EventTick
  (params (DeltaSeconds :type Float%20%28single-precision%29))
  (bind _returnvalue (Transformation|GetActorLocation))
  (bind _returnvalue_2 (Transformation|GetActorForwardVector))
  (bind _returnvalue_3 (* _returnvalue_2 1e+02))
  (bind _returnvalue_4 (+ _returnvalue_3 _returnvalue))
  ;[0.15 0.15 0.15 0.5] Raycast
  (bind _outhit (Collision|LineTraceByChannel _returnvalue_4 (+ _returnvalue_4 (Math|Vector|MakeVector 0.0 0.0 -2e+02)) "TraceTypeQuery1" false 0 "ForOneFrame"))
  (bind _asbp_tile (Utilities|Casting|CastToBP_Tile (.HitActor (Collision|BreakHitResult _outhit)))
    (:then
      (Variables|Default|SetTargetedTIle _asbp_tile)
      (if (!= _asbp_tile (Variables|Default|GetLastTargetingTIle))
        (Development|PrintString (Utilities|GetDisplayName _asbp_tile))
        (Variables|Default|SetLastTargetingTIle _asbp_tile)))
    (:CastFailed
      (Variables|Default|SetTargetedTIle 0)
      (Variables|Default|SetLastTargetingTIle 0))))

(fn ConstructionScript)

(fn PowerUps
  (params (E_PowerUp :type E_PowerUps%20Enum :default "NewEnumerator0"))
  (switch Utilities|FlowControl|Switch|SwitchonE_PowerUps E_PowerUp
    (:NewEnumerator0
      (Variables|Default|SetDinero (+ (Variables|Default|GetDinero) 100))
      (Development|PrintString "Ganaste dierno!"))
    (:NewEnumerator1
      (Development|PrintString "Velocidad"))
    (:NewEnumerator2
      (Development|PrintString "Vida"))
    (:NewEnumerator3
      (Development|PrintString "SafePlace"))
    (:NewEnumerator4
      (Development|PrintString "Nada"))))