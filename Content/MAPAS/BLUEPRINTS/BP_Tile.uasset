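; BP_Tile is a grid tile for two player boards that highlights on selection and can hold one tower.
; Initialize attaches it to its owner, sets the mesh and positions it from row/column coordinates and mesh bounds.
; OnInteract tints a dynamic material and, on selection, spawns a tower if tile type allows, then prints orthogonal neighbors from BP_Generator.
; IsWalkable box-traces from above to detect blockers, with persistent debug drawing.
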(event EventBeginPlay
  (Setup|CreateMID))

(event Collision|EventActorBeginOverlap
  (params (OtherActor :type Actor%20Object%20Reference)))

(event EventTick
  (params (DeltaSeconds :type Float%20%28single-precision%29)))

(fn ConstructionScript
  (bind _coordinates (Variables|Info|GetCoordinates))
  (Rendering|Components|TextRender|SetText (Variables|Default|GetTXT_Coordinate) (Utilities|Text|ToText(String) (Utilities|String|Append "R:" (Utilities|String|ToString(Integer) (.row _coordinates)) " 
C:" (Utilities|String|ToString(Integer) (.column _coordinates))))))

(fn Initialize
  (params (InType :type E_GridType%20Enum :default "NewEnumerator0"))
  (bind _returnvalue (Components|GetOwner))
  (Utilities|IsValid _returnvalue
    (:Is%20Valid
      (Setup|SetMesh InType)
      (Transformation|AttachActorToActor _returnvalue "None" "SnapToTarget" "SnapToTarget" "KeepRelative" false)
      (bind _outlocation (Setup|CalculateLocation InType))
      (Transformation|SetActorRelativeLocation _outlocation))))

(fn SetMesh
  (params (InType :type E_GridType%20Enum :default "NewEnumerator0"))
  (Components|StaticMesh|SetStaticMesh (Variables|Default|GetTile) (Utilities|Select :Index InType :NewEnumerator0 "/Game/MAPAS/ASSETS/MESHES/SM_TilePlayer1.SM_TilePlayer1" :NewEnumerator1 "/Game/MAPAS/ASSETS/MESHES/SM_TilePlayer1.SM_TilePlayer1"))
  (Setup|CreateMID))

(fn CalculateLocation
  (params (InType :type E_GridType%20Enum :default "NewEnumerator0"))
  (bind _tile (Variables|Default|GetTile))
  (bind _tile_2 (Variables|Default|GetTile))
  (bind _coordinates (Variables|Info|GetCoordinates))
  (bind _coordinates_2 (Variables|Info|GetCoordinates))
  (bind _boxextent (Collision|GetComponentBounds _tile_2))
  (bind _boxextent_2 (Collision|GetComponentBounds _tile))
  (bind (_x _y) (Math|Vector|BreakVector _boxextent))
  (bind (_x_2 _y_2) (Math|Vector|BreakVector _boxextent_2))
  (return (Utilities|Select :Index InType :NewEnumerator0 (Math|Vector|MakeVector (* _x (.column _coordinates) 2.0) (* _y (.row _coordinates) 2.0) 0.0) :NewEnumerator1 (Math|Vector|MakeVector (* _x_2 (.column _coordinates_2) 2.0) (* _y_2 (.row _coordinates_2) 2.0) 0.0))))

(fn IsWalkable
  (params (InType :type E_GridType%20Enum :default "NewEnumerator0"))
  (switch Utilities|FlowControl|Switch|SwitchonE_GridType InType
    (:NewEnumerator0
      (return (not (.bSuccess (Trace|TraceonBox)))))
    (:NewEnumerator1
      (return (not (.bSuccess (Trace|TraceonBox)))))))

(fn CreateMID
  (bind _returnvalue (Rendering|Material|CreateDynamicMaterialInstance (Variables|Default|GetTile) 0 "/Game/MAPAS/ASSETS/MATERIALS/M_Tile.M_Tile" "None" :!class /Script/Engine.PrimitiveComponent))
  (bind _output_get (Variables|Material|SetMID _returnvalue))
  (Rendering|Material|SetVectorParameterValue _output_get "Color" (Variables|Color|GetNormalColor) :!class /Script/Engine.MaterialInstanceDynamic))

(fn TraceonBox
  (bind (_outhit _returnvalue) (Collision|BoxTraceByChannel (Trace|GetTraceStartLocation) (Transformation|GetActorLocation) (* (+ (.BoxExtent (Collision|GetComponentBounds (Variables|Default|GetTile))) "0.000000,0.000000,30.000000") 0.9) "0, 0, 0" "TraceTypeQuery1" false (Utilities|Array|MakeArray self) "Persistent"))
  (return _returnvalue _outhit))

(fn GetTraceStartLocation
  (return (+ (Transformation|GetActorLocation) "0.000000,0.000000,150.000000")))

(fn ColocarTorre
  (Utilities|IsValid (Variables|Default|GetTorreActual)
    (:Is%20Not%20Valid
      (if (Utilities|Enum|Equal(Enum) (Variables|Default|GetTipoTile) "NewEnumerator1")
        (bind _returnvalue (Game|SpawnActorfromClass "/Game/TORRE/BP_torre.BP_torre_C" (Transformation|GetActorTransform) "AlwaysSpawn" "MultiplyWithRoot" 0 0))
        (Variables|Default|SetTorreActual _returnvalue)))))

(fn OnInteract
  (params (bInSelect :type Boolean))
  (bind _mid (Variables|Material|GetMID)
    (:then
      (Rendering|Material|SetVectorParameterValue _mid "Color" (Math|Color|SelectColor (Variables|Color|GetSelectedColor) (Variables|Color|GetNormalColor) bInSelect) :!class /Script/Engine.MaterialInstanceDynamic)
      (if bInSelect
        (CallFunction|ColocarTorre)
        (bind _asbp_generator (Utilities|Casting|CastToBP_Generator (Components|GetOwner)))
        (for _array_element (Default|GetTileNeighbors _asbp_generator self false)
          (Development|PrintString (Utilities|String|Append "R:" (Utilities|String|ToString(Integer) (.row (Variables|BP_Tile_C|GetCoordinates _array_element))) "C:" (Utilities|String|ToString(Integer) (.column (Variables|BP_Tile_C|GetCoordinates _array_element))))))))
    (:else
      (return false))))